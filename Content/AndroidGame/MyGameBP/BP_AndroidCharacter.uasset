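; Player character for a touch-screen game, with joystick-driven movement, a toggleable sprint and swipe-to-look camera control.
; Movement axes follow control yaw, and MoveForward sets the walk speed from the sprint flag.
; A touch press opens a gate polled every tick, turning finger movement beyond a swipe threshold into yaw and pitch input; nothing closes it.
; BeginPlay activates the left virtual joystick and adds the player controller widget to the viewport.
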(fn `UserConstructionScript`)